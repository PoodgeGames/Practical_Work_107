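; AI-controlled pawn that wanders randomly inside a rectangle set by Xmin/Xmax and Ymin/Ymax.
; LadaMove runs on BeginPlay, a looping two-second timer and every capsule hit, picking a random point at the pawn's height.
; PointNormal flags out-of-bounds points for a recursive retry; otherwise AIMoveTo heads there and a debug sphere marks the target.
; Tick outlines the rectangle with debug lines through the Vector2D and DebagLine helpers.
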(event OnComponentHit(CapsuleComponent)
  (params (HitComponent :type Primitive%20Component%20Object%20Reference) (OtherActor :type Actor%20Object%20Reference) (OtherComp :type Primitive%20Component%20Object%20Reference) (NormalImpulse :type Vector :default "0, 0, 0") (Hit :type Hit%20Result%20Structure%20%28by%20ref%29))
  (CallFunction|LadaMove))

(event Custom|LadaMove
  (bind _returnvector (CallFunction|PointLook))
  (bind _newparam (CallFunction|PointNormal))
  (if _newparam
    (CallFunction|LadaMove)
    (else
      (AI|AIMoveTo self _returnvector 0 5e+01 false
        (:then
          (Rendering|Debug|DrawDebugSphere (Variables|Default|GetTargetLocation) 1e+01 1 "(R=0.000000,G=0.009654,B=1.000000,A=1.000000)" 6e+01))))))

(event EventBeginPlay
  (CallFunction|LadaMove)
  (Utilities|Time|SetTimerbyEvent (delegate Custom|LadaMove) 2.0 true))

(event EventTick
  (params (DeltaSeconds :type Float%20%28single-precision%29))
  (bind (_xyminmin _xyminmax _xymaxmax _xymaxmin) (CallFunction|Vector2D))
  (CallFunction|DebagLine _xyminmin _xyminmax _xymaxmax _xymaxmin))

(fn ConstructionScript)

(fn PointLook
  (bind _output_get (Variables|Default|SetTargetLocation (Math|Vector|MakeVector (Math|Random|RandomFloatinRange (Variables|Default|GetXmin) (Variables|Default|GetXmax)) (Math|Random|RandomFloatinRange (Variables|Default|GetYmin) (Variables|Default|GetYmax)) (.z (Transformation|GetActorLocation)))))
  (return _output_get))

(fn PointNormal
  (return (Math|Boolean|ORBoolean (> (.x (Variables|Default|GetTargetLocation)) (Variables|Default|GetXmax)) (> (.y (Variables|Default|GetTargetLocation)) (Variables|Default|GetYmax)) (< (.x (Variables|Default|GetTargetLocation)) (Variables|Default|GetXmin)) (< (.y (Variables|Default|GetTargetLocation)) (Variables|Default|GetYmin)))))

(fn Vector2D
  (bind _output_get (Variables|Default|SetXYMinMin (Math|Vector2D|MakeVector2D (Variables|Default|GetXmin) (Variables|Default|GetYmin))))
  (bind _output_get_2 (Variables|Default|SetXYMinMax (Math|Vector2D|MakeVector2D (Variables|Default|GetXmin) (Variables|Default|GetYmax))))
  (bind _output_get_3 (Variables|Default|SetXYMaxMax (Math|Vector2D|MakeVector2D (Variables|Default|GetXmax) (Variables|Default|GetYmax))))
  (bind _output_get_4 (Variables|Default|SetXYMaxMin (Math|Vector2D|MakeVector2D (Variables|Default|GetXmax) (Variables|Default|GetYmin))))
  (return _output_get _output_get_2 _output_get_3 _output_get_4))

(fn DebagLine
  (params (PointA :type Vector%202D%20Structure) (PointB :type Vector%202D%20Structure) (PointC :type Vector%202D%20Structure) (PointD :type Vector%202D%20Structure))
  (Rendering|Debug|DrawDebugLine (Math|Conversions|ToVector(Vector2D) PointA 3e+01) (Math|Conversions|ToVector(Vector2D) PointB 3e+01) "(R=1.000000,G=0.058392,B=0.000000,A=1.000000)" 0.0 3.0)
  (Rendering|Debug|DrawDebugLine (Math|Conversions|ToVector(Vector2D) PointC 3e+01) (Math|Conversions|ToVector(Vector2D) PointD 3e+01) "(R=1.000000,G=0.058392,B=0.000000,A=1.000000)" 0.0 3.0)
  (Rendering|Debug|DrawDebugLine (Math|Conversions|ToVector(Vector2D) PointC 3e+01) (Math|Conversions|ToVector(Vector2D) PointB 3e+01) "(R=1.000000,G=0.058392,B=0.000000,A=1.000000)" 0.0 3.0)
  (Rendering|Debug|DrawDebugLine (Math|Conversions|ToVector(Vector2D) PointD 3e+01) (Math|Conversions|ToVector(Vector2D) PointA 3e+01) "(R=1.000000,G=0.058392,B=0.000000,A=1.000000)" 0.0 3.0))